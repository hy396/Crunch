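; Projectile actor for Reimu's shoot ability that takes on a random visual variant each time it spawns.
; On BeginPlay it rolls one index into the Effects array, applying that particle template and the matching hit GameplayCue tag.
; SpawnExplosion reuses the index to spawn the paired explosion emitter at the actor's location, so parallel arrays keep trail, hit cue and explosion consistent.
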(event `self.ReceiveBeginPlay`
  (bind _output_get (set `self.Index` (`KismetMathLibrary.RandomIntegerInRange` 0 (- (`KismetArrayLibrary.Array_Length` (`self.Effects`)) 1))))
  (`ParticleSystemComponent.SetTemplate` (`self.ParticleSystem`) (`|GetArrayItem` (`self.Effects`) _output_get))
  (`self.SetHitGameplayCueTag` (`|GetArrayItem` (`self.HitGameplayCueTags`) (`self.Index`))))

(event `self.SpawnExplosion`
  (`GameplayStatics.SpawnEmitterAtLocation` (`|GetArrayItem` (`self.Explosions`) (`self.Index`)) (`self.K2_GetActorLocation`)))

(fn `UserConstructionScript`)