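; Main menu player controller that boots the frontend UI for the local player.
; After a short delay on BeginPlay, it creates the primary layout widget, adds it to the viewport and registers it with the frontend UI subsystem.
; It then pushes the tag-resolved Press Any Key soft widget class onto the Frontend widget stack, printing a debug string afterwards.
; Tick and Possess are empty; an authority test is left unwired.
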(event `self.ReceiveBeginPlay`
  (if (`self.IsLocalPlayerController`)
    (`KismetSystemLibrary.Delay` 0.2)
    (bind _returnvalue (`|CreateWidget` "/Game/Widgets/FrontendUI/Widgets/WBP_CUW_PrimaryLayout.WBP_CUW_PrimaryLayout_C" self))
    (`UserWidget.AddToViewport` _returnvalue 0)
    (`FrontendUISubsystem.RegisterCreatedPrimaryLayoutWidget` (subsystem `FrontendUISubsystem`) _returnvalue)
    (`AsyncAction_PushSoftWidget.PushSoftWidget` self (`FrontendFunctionLibrary.GetFrontendSoftWidgetClassByTag` (struct :`TagName` "Frontend.Widget.PressAnyKeyScreen")) (struct :`TagName` "Frontend.WidgetStack.Frontend")
      (:`AfterPush`
        (`KismetSystemLibrary.PrintString` "OJBK")))))

(event `self.ReceivePossess`
  (params (PossessedPawn :type "Pawn Object Reference"))
  ;[1 1 1] OnPosses是在服务器执行的，客户端不打印
)

(fn `UserConstructionScript`)