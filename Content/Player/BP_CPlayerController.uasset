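; BP_CPlayerController is the player controller that sets up input and the root frontend UI layout when play begins.
; For the local controller, it registers gameplay and controller input mapping contexts with Enhanced Input user settings.
; It also creates the primary layout widget, adds it to the viewport and registers it with the FrontendUI subsystem.
; It then stops the seamless loading screen; a confirm-screen test is left unconnected.
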(event `self.ReceiveBeginPlay`
  (bind _returnvalue (`EnhancedInputSubsystemInterface.GetUserSettings` (subsystem `EnhancedInputLocalPlayerSubsystem`)))
  (`|ExecutionSequence`
    (:`then_0`
      (if (`self.IsLocalPlayerController`)
        (`EnhancedInputUserSettings.RegisterInputMappingContext` _returnvalue "/Game/Input/IMC_Gameplay.IMC_Gameplay")
        (`EnhancedInputUserSettings.RegisterInputMappingContext` _returnvalue "/Game/Input/IMC_PlayerController.IMC_PlayerController")
        (bind _returnvalue_2 (`|CreateWidget` "/Game/Widgets/FrontendUI/Widgets/WBP_CUW_PrimaryLayout.WBP_CUW_PrimaryLayout_C" self))
        (`UserWidget.AddToViewport` _returnvalue_2 1)
        (`FrontendUISubsystem.RegisterCreatedPrimaryLayoutWidget` (subsystem `FrontendUISubsystem`) _returnvalue_2)))
    (:`then_1`
      (`AsyncLoadingScreenLibrary.StopSeamlessLoadingScreen`))))

(fn `UserConstructionScript`)